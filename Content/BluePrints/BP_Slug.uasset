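; BP_Slug is an enemy slug that homes in on the player character and fires at them on a looping timer.
; Each tick it eases its yaw toward the player with RInterpTo and teleports toward them without sweeping.
; Shots are enlarged, cobblestone-skinned FirstPersonProjectiles with explosion effect and sound.
; On Hit, a projectile destroys it with an explosion, while touching the player calls HealthController.DecreaseHealth.
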(event `self.ReceiveTick`
  (params (DeltaSeconds :type "Float (single-precision)"))
  (bind _rotation (`self.GetMainCharacterRotation`))
  (`self.K2_SetActorRotation` _rotation true)
  (`self.MoveToMainCharacter` DeltaSeconds))

(event `self.ReceiveBeginPlay`
  (`SkeletalMeshComponent.PlayAnimation` (`self.SkeletalMesh`) "/Game/Models/Slug/slug_Anim_Idle.slug_Anim_Idle" true)
  (`KismetSystemLibrary.K2_SetTimer` null "ShootMainCharacter" (`self.FireTimeInterval`) true))

(event `self.ReceiveHit`
  (params (MyComp :type "PrimitiveComponent Object Reference") (Other :type "Actor Object Reference") (OtherComp :type "PrimitiveComponent Object Reference") (bSelfMoved :type Boolean) (HitLocation :type "Vector Structure") (HitNormal :type "Vector Structure") (NormalImpulse :type "Vector Structure") (Hit :type "HitResult Structure (by ref)"))
  (`self.CheckAndDestroy` HitLocation Other))

(fn `CheckAndDestroy`
  (params (HitLocation :type "Vector Structure") (OtherActor :type "Actor Object Reference"))
  ;[1 1 1] Only can be destroyed by projectiles and mobile cubes
  (cast `/Game/FirstPersonBP/Blueprints/FirstPersonProjectile` OtherActor
    (:`then`
      (`GameplayStatics.SpawnEmitterAtLocation` "/Game/StarterContent/Particles/P_Explosion.P_Explosion" HitLocation)
      (`self.K2_DestroyActor`)
      ;[1 1 1] No more enemies
      (bind _outactors (`GameplayStatics.GetAllActorsOfClass` "BP_Slug_C"))
      (if (== (`KismetArrayLibrary.Array_Length` _outactors) 0)
        _))
    (:`CastFailed`
      (cast `/Game/FirstPersonBP/Blueprints/FirstPersonCharacter` OtherActor)
      (`HealthController.decreaseHealth` (`self.HealthController`) 1))))

(fn `Get_Look_At_Rotation`
  (params (MyActor :type "Actor Object Reference") (Target :type "Actor Object Reference"))
  (returns (ReturnValue :type "Rotator Structure"))
  (return (`KismetMathLibrary.RInterpTo` (`self.K2_GetActorRotation` MyActor) (`KismetMathLibrary.MakeRotator` 0.0 0.0 (.yaw (`KismetMathLibrary.FindLookAtRotation` (`self.K2_GetActorLocation` MyActor) (`self.K2_GetActorLocation` Target)))) (`GameplayStatics.GetWorldDeltaSeconds`) 3.0)))

(fn `GetMainCharacterRotation`
  (returns (Rotation :type "Rotator Structure"))
  (bind _asfirst_person_character (cast `/Game/FirstPersonBP/Blueprints/FirstPersonCharacter` (`GameplayStatics.GetPlayerCharacter` 0)))
  (bind _returnvalue (`self.Get_Look_At_Rotation` self _asfirst_person_character))
  (return _returnvalue))

(fn `MoveToMainCharacter`
  (params (DeltaSeconds :type "Float (double-precision)"))
  (`self.K2_SetActorTransform` (`KismetMathLibrary.MakeTransform` (+ (* (* (`KismetMathLibrary.Normal` (- (`self.K2_GetActorLocation`) (`self.K2_GetActorLocation` (`GameplayStatics.GetPlayerPawn` 0)))) -1.0) (* DeltaSeconds (`self.Speed`))) (.location (`SceneComponent.K2_GetComponentToWorld` (`self.SkeletalMesh`)))) (.rotation (`SceneComponent.K2_GetComponentToWorld` (`self.SkeletalMesh`))) (.scale (`SceneComponent.K2_GetComponentToWorld` (`self.SkeletalMesh`)))) false true))

(fn `ShootMainCharacter`
  (bind _rotation (.rotation (`self.GetTransform`)))
  (bind _returnvalue (+ (.location (`self.GetTransform`)) (0.0 0.0 150.0)))
  (`GameplayStatics.SpawnEmitterAtLocation` "/Game/StarterContent/Particles/P_Explosion.P_Explosion" _returnvalue _rotation)
  (bind _returnvalue_2 (`|SpawnActorFromClass` "/Game/FirstPersonBP/Blueprints/FirstPersonProjectile.FirstPersonProjectile_C" (`KismetMathLibrary.MakeTransform` _returnvalue _rotation (3.0 3.0 3.0)) "Undefined" "OverrideRootScale" null null))
  (`PrimitiveComponent.SetMaterial` (`/Game/FirstPersonBP/Blueprints/FirstPersonProjectile.Sphere` _returnvalue_2) 0 "/Game/StarterContent/Materials/M_CobbleStone_Smooth.M_CobbleStone_Smooth")
  (`GameplayStatics.PlaySoundAtLocation` "/Game/StarterContent/Audio/Explosion_Cue.Explosion_Cue" (`self.K2_GetActorLocation`)))

(fn `UserConstructionScript`)